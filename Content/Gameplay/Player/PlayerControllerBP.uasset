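; Player controller for the robot character, managing camera, pause menu, audio attenuation and AI damage reporting.
; Tick eases the spring arm toward the newest follow-camera volume's distance and rotation, and blends to the top of a view-target stack, falling back to the pawn.
; Both camera systems snap on their first update.
; Debug keys for baby, knockdown and save actions work outside distribution builds, while quit and reset keys require the pause screen.
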(event `Key|Subtract`
  (params (Key :type "Key Structure"))
  (bind _baby (`/Game/Gameplay/HelperFunctions.GetActiveBaby`))
  ;[1 1 1] DebugInput
  (:`Pressed`
    (`self.DebugExec`
      (:`Out`
        (`/Engine/EditorBlueprintResources/StandardMacros.IsValid` _baby
          (:`Is Valid`
            (`/Game/Gameplay/Baby/BabyActor.SetBabyClock` _baby (- (`/Game/Gameplay/Baby/BabyActor.BabyClock` _baby) 10.0))))))))

(event `PushFollowCameraVolume`
  (params (FollowCameraVolume :type "/Game/Gameplay/Camera/FollowCameraBox Object Reference"))
  (`KismetArrayLibrary.Array_Add` (`self.FollowCameraVolumes`) FollowCameraVolume))

(event `Key|Add`
  (params (Key :type "Key Structure"))
  (bind _baby (`/Game/Gameplay/HelperFunctions.GetActiveBaby`))
  ;[1 1 1] DebugInput
  (:`Pressed`
    (`self.DebugExec`
      (:`Out`
        (`/Engine/EditorBlueprintResources/StandardMacros.IsValid` _baby
          (:`Is Valid`
            (`/Game/Gameplay/Baby/BabyActor.SetBabyClock` _baby (+ (`/Game/Gameplay/Baby/BabyActor.BabyClock` _baby) 10.0))))))))

(event `RemoveFollowCameraVolume`
  (params (FollowCameraVolume :type "/Game/Gameplay/Camera/FollowCameraBox Object Reference"))
  (bind _followcameravolumes (`self.FollowCameraVolumes`))
  (bind _followcameravolumes_2 (`self.FollowCameraVolumes`))
  (bind _returnvalue (`KismetArrayLibrary.Array_Find` _followcameravolumes_2 FollowCameraVolume))
  (if (`KismetArrayLibrary.Array_IsValidIndex` _followcameravolumes_2 _returnvalue)
    (`KismetArrayLibrary.Array_Remove` _followcameravolumes _returnvalue)
    (if (> (`KismetArrayLibrary.Array_Length` _followcameravolumes) 0)
      _)))

(event `Key|B`
  (params (Key :type "Key Structure"))
  (bind _baby (`/Game/Gameplay/HelperFunctions.GetActiveBaby`))
  ;[1 1 1] DebugInput
  (:`Pressed`
    (`self.DebugExec`
      (:`Out`
        (`/Engine/EditorBlueprintResources/StandardMacros.IsValid` (`/Game/Gameplay/HelperFunctions.GetActiveBaby`)
          (:`Is Valid`
            _)
          (:`Is Not Valid`
            (`|SpawnActorFromClass` "/Game/Gameplay/Baby/BabyActor.BabyActor_C" (`self.GetTransform` (`/Game/Gameplay/HelperFunctions.GetRobotCharacter`)) "Undefined" "OverrideRootScale" null null)))
        (`/Game/Gameplay/Baby/BabyActor.PickupBaby` _baby (`/Game/Gameplay/HelperFunctions.GetRobotCharacter`))
        (`/Game/Gameplay/Baby/BabyActor.TickBabyAttachLerp` _baby 9999.0)))))

(event `PushViewTarget`
  (params (Target :type "Actor Object Reference") (Transition :type "ViewTargetTransitionParams Structure"))
  (`KismetArrayLibrary.Array_Add` (`self.ViewTargets`) Target)
  (`KismetArrayLibrary.Array_Add` (`self.ViewTargetTransitions`) Transition))

(event `Key|BackSpace`
  (params (Key :type "Key Structure"))
  ;[1 1 1] DebugInput
  (:`Pressed`
    (`self.DebugExec`
      (:`Out`
        (`/Game/Gameplay/HelperFunctions.LoadGame` false)))))

(event `Key|Ctrl+BackSpace`
  (params (Key :type "Key Structure"))
  ;[1 1 1] DebugInput
  (:`Pressed`
    (`self.DebugExec`
      (:`Out`
        (`/Game/Gameplay/HelperFunctions.ResetGame` false)))))

(event `Key|K`
  (params (Key :type "Key Structure"))
  ;[1 1 1] DebugInput
  (:`Pressed`
    (`self.DebugExec`
      (:`Out`
        (`/Game/Gameplay/Player/RobotPlayerCharacter.Knockdown` (`/Game/Gameplay/HelperFunctions.GetRobotCharacter`) (0.0 0.0 0.0))))))

(event `RemoveViewTarget`
  (params (Target :type "Actor Object Reference"))
  (bind _viewtargets (`self.ViewTargets`))
  (bind _returnvalue (`KismetArrayLibrary.Array_Find` _viewtargets Target))
  (if (`KismetArrayLibrary.Array_IsValidIndex` _viewtargets _returnvalue)
    (`KismetArrayLibrary.Array_Remove` (`self.ViewTargets`) _returnvalue)
    (`KismetArrayLibrary.Array_Remove` (`self.ViewTargetTransitions`) _returnvalue)))

(event `InputAction|Pause` :paused true
  (params (Key :type "Key Structure"))
  (bind _pausescreen (`self.PauseScreen`))
  (:`Pressed`
    (`/Engine/EditorBlueprintResources/StandardMacros.IsValid` _pausescreen
      (:`Is Valid`
        (`/Game/Gameplay/UI/PauseScreen.ExitPauseScreen` _pausescreen))
      (:`Is Not Valid`
        (bind _returnvalue (`|CreateWidget` "/Game/Gameplay/UI/PauseScreen.PauseScreen_C" self))
        (`UserWidget.AddToPlayerScreen` _returnvalue 99)
        (bind _output_get (set `self.PauseScreen` _returnvalue))
        (add `/Game/Gameplay/UI/PauseScreen.ExitEvent` _output_get (delegate `OnPauseMenuExit`))))))

(event `OnPauseMenuExit`
  (set `self.PauseScreen` null))

(event `Key|Q` :paused true
  (params (Key :type "Key Structure"))
  (:`Pressed`
    (`/Engine/EditorBlueprintResources/StandardMacros.IsValid` (`self.PauseScreen`)
      (:`Is Valid`
        (`KismetSystemLibrary.QuitGame` null "Quit")))))

(event `Key|R` :paused true
  (params (Key :type "Key Structure"))
  (:`Pressed`
    (`/Engine/EditorBlueprintResources/StandardMacros.IsValid` (`self.PauseScreen`)
      (:`Is Valid`
        (`/Game/Gameplay/HelperFunctions.ResetGame` true)))))

(event `self.ReceiveTick`
  (params (DeltaSeconds :type "Float (single-precision)"))
  (`self.TickFollowCameraVolumes` DeltaSeconds)
  (`self.TickViewTargetStack`))

(event `self.ReceiveInstigatedAnyDamage`
  (params (Damage :type "Float (single-precision)") (DamageType :type "DamageType Object Reference") (DamagedActor :type "Actor Object Reference") (DamageCauser :type "Actor Object Reference"))
  (bind _returnvalue (`self.K2_GetActorLocation` DamagedActor))
  (`AISense_Damage.ReportDamageEvent` DamagedActor self Damage _returnvalue _returnvalue))

(event `self.ReceivePossess`
  (params (PossessedPawn :type "Pawn Object Reference"))
  (`self.SetAudioListenerAttenuationOverride` (`Actor.RootComponent` PossessedPawn)))

(fn `TickFollowCameraVolumes`
  (params (DeltaTime :type "Float (double-precision)"))
  (locals (DistanceTarget :type "Float (double-precision)" :default 2000.0) (DistanceSpeed :type "Float (double-precision)" :default 5000.0) (RotTarget :type "Rotator Structure" :default (struct :`Pitch` -45.0)) (RotSpeed :type "Float (double-precision)" :default 360.0))
  (bind _followcameravolumes (`self.FollowCameraVolumes`))
  (bind _output (`|GetArrayItem` _followcameravolumes (`KismetArrayLibrary.Array_LastIndex` _followcameravolumes)))
  (`|ExecutionSequence`
    (:`then_0`
      (if (> (`KismetArrayLibrary.Array_Length` (`self.FollowCameraVolumes`)) 0)
        (set `local.DistanceTarget` (`/Game/Gameplay/Camera/FollowCameraBox.Distance` _output))
        (set `local.DistanceSpeed` (`/Game/Gameplay/Camera/FollowCameraBox.DistanceBlendSpeed` _output))
        (set `local.RotTarget` (`/Game/Gameplay/Camera/FollowCameraBox.Rot` _output))
        (set `local.RotSpeed` (`/Game/Gameplay/Camera/FollowCameraBox.RotBlendSpeed` _output))))
    (:`then_1`
      (if (not (`self.HasInitalisedFollowCamera`))
        (set `self.HasInitalisedFollowCamera` true)
        (set `local.DistanceSpeed` 999999.0)
        (set `local.RotSpeed` 999999.0)))
    (:`then_2`
      (bind _asrobot_player_character (cast `/Game/Gameplay/Player/RobotPlayerCharacter` (`self.K2_GetPawn`)))
      (bind _springarm (`/Game/Gameplay/Player/RobotPlayerCharacter.SpringArm` _asrobot_player_character))
      (set `SpringArmComponent.TargetArmLength` (`KismetMathLibrary.FInterpTo_Constant` (`SpringArmComponent.TargetArmLength` _springarm) (`local.DistanceTarget`) (`local.DeltaTime`) (`local.DistanceSpeed`)) _springarm)
      (`SceneComponent.K2_SetWorldRotation` _springarm (`KismetMathLibrary.RInterpTo_Constant` (`SceneComponent.K2_GetComponentRotation` _springarm) (`local.RotTarget`) (`local.DeltaTime`) (`local.RotSpeed`)) false false))))

(fn `TickViewTargetStack`
  (bind _viewtargets (`self.ViewTargets`))
  (bind _returnvalue (`KismetArrayLibrary.Array_LastIndex` (`self.ViewTargets`)))
  (bind _output (`|GetArrayItem` (`self.ViewTargets`) _returnvalue))
  (bind (_blendtime _blendfunction _blendexp _blockoutgoing) (break `ViewTargetTransitionParams` (`|GetArrayItem` (`self.ViewTargetTransitions`) _returnvalue)))
  (`|ExecutionSequence`
    (:`then_0`
      (if (> (`KismetArrayLibrary.Array_Length` _viewtargets) 0)
        (if (!= (`|GetArrayItem` _viewtargets (`KismetArrayLibrary.Array_LastIndex` _viewtargets)) (`self.GetViewTarget`))
          (if (`self.HasInitialisedViewTarget`)
            (`self.SetViewTargetWithBlend` _output _blendtime _blendfunction _blendexp _blockoutgoing)
            (else
              (`self.SetViewTargetWithBlend` _output 0.0 "VTBlend_Linear" 0.0 true))))
        (elif (!= (`self.K2_GetPawn`) (`self.GetViewTarget`))
          (`self.SetViewTargetWithBlend` (`self.K2_GetPawn`) 0.5 "VTBlend_Linear" 0.0 true))))
    (:`then_1`
      (set `self.HasInitialisedViewTarget` true))))

(fn `UserConstructionScript`)