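; Game mode that runs the game's flow through Title, Playing, Game Over and End states, with pausing, robot input, screen widgets and theme music.
; ChangeState handles exit and entry per state; widget exit events start play, reload the level or reset the game.
; A GameInstance flag limits the title screen, with a respawn screen shown otherwise.
; FindPlayerStart prefers play-from-here, then starting incubator, then "GameStart" tag; RegisterBaby tracks one active baby.
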(event `self.ReceiveBeginPlay`
  (bind _incubator (`/Game/Gameplay/HelperFunctions.FindStartingIncubator` true))
  (`|ExecutionSequence`
    (:`then_0`
      (bind _asgame_instance_bp (cast `/Game/GameInstanceBP` (`GameplayStatics.GetGameInstance`)))
      (if (`/Game/GameInstanceBP.ShowTitleScreen` _asgame_instance_bp)
        (`self.ChangeState` "NewEnumerator1")
        (else
          (`self.ChangeState` "NewEnumerator2")
          (bind _returnvalue (`|CreateWidget` "/Game/Gameplay/UI/RespawnScreen.RespawnScreen_C" (`GameplayStatics.GetPlayerController` 0)))
          (`UserWidget.AddToPlayerScreen` _returnvalue 0))))
    (:`then_1`
      (bind _returnvalue_2 (`|CreateWidget` "/Game/Gameplay/UI/HUDWidget.HUDWidget_C" (`GameplayStatics.GetPlayerController` 0)))
      (`UserWidget.AddToPlayerScreen` _returnvalue_2 0))
    (:`then_2`
      (`/Engine/EditorBlueprintResources/StandardMacros.IsValid` _incubator
        (:`Is Valid`
          (`/Game/Gameplay/Incubator/IncubatorActor.OnSpawnHere` _incubator))))))

(event `ChangeState`
  (params (NewState :type "/Game/Gameplay/GameModeState Enum" :default "NewEnumerator0"))
  (bind _robot (`/Game/Gameplay/HelperFunctions.GetRobotCharacter`))
  (bind _robot_2 (`/Game/Gameplay/HelperFunctions.GetRobotCharacter`))
  (if (!= NewState (`self.ModeState`))
    (`|ExecutionSequence`
      (:`then_0`
        (switch `/Game/Gameplay/GameModeState` (`self.ModeState`)
          (:`NewEnumerator2`
            (`GameplayStatics.SetGamePaused` false)
            (`self.DisableInput` _robot_2 null)
            (`Controller.SetIgnoreMoveInput` (`Pawn.GetController` _robot_2) true))))
      (:`then_1`
        (bind _output_get (set `self.ModeState` NewState))
        (switch `/Game/Gameplay/GameModeState` _output_get
          (:`NewEnumerator1`
            (`GameplayStatics.SetGamePaused` true)
            (bind _returnvalue (`|CreateWidget` "/Game/Gameplay/UI/TitleScreenWidget.TitleScreenWidget_C" (`GameplayStatics.GetPlayerController` 0)))
            (bind _output_get_2 (set `self.TitleWidget` _returnvalue))
            (add `/Game/Gameplay/UI/TitleScreenWidget.ExitEvent` _output_get_2 (delegate `TitleScreenExit`))
            (`UserWidget.AddToPlayerScreen` _output_get_2 1)
            (bind _asgame_instance_bp (cast `/Game/GameInstanceBP` (`GameplayStatics.GetGameInstance`)))
            (set `/Game/GameInstanceBP.ShowTitleScreen` false _asgame_instance_bp))
          (:`NewEnumerator2`
            (`GameplayStatics.SetGamePaused` false)
            (`self.EnableInput` _robot null)
            (`Controller.SetIgnoreMoveInput` (`Pawn.GetController` _robot) false)
            (`KismetSystemLibrary.Delay` 2.0)
            (bind _returnvalue_2 (`GameplayStatics.SpawnSound2D` "/Game/Audio/Assets/Music/Game_Theme_Loop_v3.Game_Theme_Loop_v3" 1.0 1.0 0.0 null)))
          (:`NewEnumerator4`
            (`GameplayStatics.SetGamePaused` false)
            (bind _returnvalue_3 (`|CreateWidget` "/Game/Gameplay/UI/GameOverScreen.GameOverScreen_C" (`GameplayStatics.GetPlayerController` 0)))
            (bind _output_get_3 (set `self.GameOverWidget` _returnvalue_3))
            (`UserWidget.AddToPlayerScreen` _output_get_3 1)
            (add `/Game/Gameplay/UI/GameOverScreen.ExitEvent` (`self.GameOverWidget`) (delegate `OnGameOverExit`))
            (if (`AudioComponent.IsPlaying` _returnvalue_2) :!label _label
              (`AudioComponent.FadeOut` _returnvalue_2 2.0 0.0 "Linear")))
          (:`NewEnumerator3`
            (`GameplayStatics.SetGamePaused` true)
            (bind _returnvalue_4 (`|CreateWidget` "/Game/Gameplay/UI/EndGameScreen.EndGameScreen_C" (`GameplayStatics.GetPlayerController` 0)))
            (`UserWidget.AddToPlayerScreen` _returnvalue_4 1)
            (add `/Game/Gameplay/UI/EndGameScreen.ExitEvent` _returnvalue_4 (delegate `EndGameExit`))
            (goto _label)))))))

(event `TitleScreenExit`
  (`self.ChangeState` "NewEnumerator2")
  (`GameplayStatics.SpawnSound2D` "/Game/Audio/Assets/UI_HUD/Pressstrt.Pressstrt" 1.0 1.0 0.0 null))

(event `OnMediaEnd`
  (switch `/Game/Gameplay/GameModeState` (`self.ModeState`)
    (:`NewEnumerator1`
      (`self.ChangeState` "NewEnumerator2"))))

(event `OnGameOverExit`
  (bind _returnvalue (`GameplayStatics.GetCurrentLevelName` true))
  (`GameplayStatics.OpenLevel` (`KismetStringLibrary.Conv_StringToName` _returnvalue)))

(event `EndGameExit`
  (`/Game/Gameplay/HelperFunctions.ResetGame` true))

(fn `FindPlayerStart`
  (params (Player :type "Controller Object Reference") (IncomingName :type String))
  (returns (ReturnValue :type "Actor Object Reference"))
  (bind _incubator (`/Game/Gameplay/HelperFunctions.FindStartingIncubator` false))
  (bind _returnvalue (`parent.FindPlayerStart` Player IncomingName))
  (bind _asplayer_start_pie (cast `PlayerStartPIE` _returnvalue)
    (:`then`
      (`|ExecutionSequence`
        (:`then_0`
          (bind _asgame_instance_bp (cast `/Game/GameInstanceBP` (`GameplayStatics.GetGameInstance`)))
          (set `/Game/GameInstanceBP.ShowTitleScreen` false _asgame_instance_bp))
        (:`then_1`
          (return _asplayer_start_pie))))
    (:`CastFailed`
      (`/Engine/EditorBlueprintResources/StandardMacros.IsValid` _incubator
        (:`Is Valid`
          (return (`ChildActorComponent.ChildActor` (`/Game/Gameplay/Incubator/IncubatorActor.PlayerStart` _incubator))))
        (:`Is Not Valid`
          (bind _outactors (`GameplayStatics.GetAllActorsOfClass` "/Script/Engine.PlayerStart"))
          (for _array_element _outactors
            (if (== (`PlayerStart.PlayerStartTag` _array_element) "GameStart")
              (return _array_element)))
          (return _returnvalue))))))

(fn `RegisterBaby`
  (params (Baby :type "/Game/Gameplay/Baby/BabyActor Object Reference"))
  (`/Engine/EditorBlueprintResources/StandardMacros.IsValid` (`self.ActiveBaby`)
    (:`Is Valid`
      (`KismetSystemLibrary.PrintString` "THERE SHOULD ONLY BE ONE ACTIVE BABY" true true (struct :`R` 1.0 :`A` 1.0) 10.0))
    (:`Is Not Valid`
      (set `self.ActiveBaby` Baby))))

(fn `UserConstructionScript`)